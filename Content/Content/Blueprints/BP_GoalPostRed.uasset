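; BP_GoalPostRed is the red goal post, which detects the football and reports a goal to the game mode.
; When BP_FootBall overlaps its S component, it spawns the Explod particle system at the ball and destroys it.
; It then clears NotPaused on BP_GameMode and, after a short delay, calls Goal with a true flag.
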(event OnComponentBeginOverlap(s)
  (params (OverlappedComponent :type Primitive%20Component%20Object%20Reference) (OtherActor :type Actor%20Object%20Reference) (OtherComp :type Primitive%20Component%20Object%20Reference) (OtherBodyIndex :type Integer) (bFromSweep :type Boolean) (SweepResult :type Hit%20Result%20Structure%20%28by%20ref%29))
  (bind _asbp_foot_ball (Utilities|Casting|CastToBP_FootBall OtherActor))
  (Niagara|SpawnSystematLocation "/Game/Content/Blueprints/Particles/Explod.Explod" (.location (Transformation|GetActorTransform _asbp_foot_ball)))
  (Actor|DestroyActor _asbp_foot_ball)
  (bind _asbp_game_mode (Utilities|Casting|CastToBP_GameMode (Game|GetGameMode)))
  (Variables|/Game/Content/Maps/GameMap/BP_GameMode.BP_GameMode_C|SetNotPaused _asbp_game_mode false)
  (Utilities|FlowControl|Delay 3.0)
  (Default|Goal _asbp_game_mode true))

(event EventBeginPlay)

(event Collision|EventActorBeginOverlap
  (params (OtherActor :type Actor%20Object%20Reference)))

(event EventTick
  (params (DeltaSeconds :type Float%20%28single-precision%29)))

(fn ConstructionScript)