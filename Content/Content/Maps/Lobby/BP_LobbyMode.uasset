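; BP_LobbyMode is the lobby game mode Blueprint that tracks connected lobby controllers in a player list.
; On post-login it adds the controller, passes the resulting list index to SetPlayerState, refreshes every controller's widget through RequestUpdate, and increments Total on the game instance.
; Logout only removes the controller from the list, with no widget refresh or change to Total.
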(event Custom|RequestUpdate
  (for _array_element (Variables|Default|GetPlayerList)
    (bind _asbp_lobby_ctrl (Utilities|Casting|CastToBP_LobbyCtrl _array_element))
    (Default|UpdateWidget _asbp_lobby_ctrl)))

(event EventPostLogin
  (params (NewPlayer :type Player%20Controller%20Object%20Reference))
  (bind _returnvalue (Utilities|Array|Add (Variables|Default|GetPlayerList) NewPlayer))
  (bind _asbp_lobby_ctrl (Utilities|Casting|CastToBP_LobbyCtrl NewPlayer))
  (Default|SetPlayerState _asbp_lobby_ctrl _returnvalue)
  (CallFunction|RequestUpdate)
  (Math|Integer|IncrementInt (Variables|/Game/Content/Blueprints/BP_GameInstance.BP_GameInstance_C|GetTotal (.AsBP%20Game%20Instance (Utilities|Casting|CastToBP_GameInstance (Game|GetGameInstance))))))

(event EventOnLogout
  (params (ExitingController :type Controller%20Object%20Reference))
  (bind _asbp_lobby_ctrl (Utilities|Casting|CastToBP_LobbyCtrl ExitingController))
  (Utilities|Array|RemoveItem (Variables|Default|GetPlayerList) _asbp_lobby_ctrl))

(fn ConstructionScript)