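; BP_GameControl is the player controller for a Blue-versus-Red team match, managing match UI, scores and input.
; SetPlayerState copies username and team from the GameInstance into BP_PlayerState, retrying each second until the cast succeeds.
; CallFromServer switches the phase: loading to HUD and countdown, score with another countdown, or winner screen with UI-only input.
; UnFreeze clears the countdown and enables pawn input, while score OnRep functions refresh the HUD.
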(event Custom|SetPlayerState
  (bind _returnvalue (Game|GetGameInstance))
  (bind _asbp_game_instance (Utilities|Casting|CastToBP_GameInstance _returnvalue))
  ;[1 1 1] Comment
  (CallFunction|CreateLoading)
  (CallFunction|SetState (Variables|/Game/Content/Blueprints/BP_GameInstance.BP_GameInstance_C|GetTeamPlayerNo _asbp_game_instance) (Variables|/Game/Content/Blueprints/BP_GameInstance.BP_GameInstance_C|GetUsername _asbp_game_instance)))

(event Custom|SetState
  (params (team :type Integer) (username :type Text))
  ;[1 1 1] Comment
  (bind _asbp_player_state (Utilities|Casting|CastToBP_PlayerState (Variables|GetPlayerState) :!label _label)
    (:then
      (Variables|/Game/Content/Maps/Lobby/BP_PlayerState.BP_PlayerState_C|Setusername _asbp_player_state username)
      (Variables|/Game/Content/Maps/Lobby/BP_PlayerState.BP_PlayerState_C|Setteam _asbp_player_state team))
    (:CastFailed
      (Utilities|FlowControl|Delay 1.0)
      (goto _label))))

(event Custom|CreateLoading
  ;[1 1 1] Loading and HUD
  (Variables|Default|GetLoadingWid
    (:then
      _)
    (:else
      (bind _returnvalue (UserInterface|CreateWidget "/Game/Content/Maps/GameMap/Loading.Loading_C"))
      (Variables|Default|SetLoadingWid _returnvalue)))
  (UserInterface|Viewport|AddtoViewport (Variables|Default|GetLoadingWid) 0))

(event Custom|CallFromServer
  (params (Team :type Boolean) (What :type Integer))
  (switch int What
    (:0
      (CallFunction|RemoveLoading)
      (CallFunction|CreateCountDown))
    (:1
      (Math|Integer|IncrementInt (select Team (Variables|Default|GetBlueScore) (Variables|Default|GetRedScore))
        (:%20%20
          (CallFunction|CreateCountDown)
          (bind _hud (Variables|Default|GetHUD)
            (:then
              (Variables|/Script/UMG.TextBlock|SetText (Variables|/Game/Content/UI/HUD.HUD_C|GetBlueScore _hud) (Utilities|Text|FormatText "Blue : {bluescore}" (Variables|Default|GetBlueScore)))
              (Variables|/Script/UMG.TextBlock|SetText (Variables|/Game/Content/UI/HUD.HUD_C|GetRedScore _hud) (Utilities|Text|FormatText "Red : {redscore}" (Variables|Default|GetRedScore))))
            (:else)))))
    (:2
      (CallFunction|GameEnd))))

(event Custom|RemoveLoading
  ;[1 1 1] Loading and HUD
  (Variables|Default|GetLoadingWid
    (:then
      (Widget|RemovefromParent (Variables|Default|GetLoadingWid))
      (Variables|Default|SetLoadingWid 0)
      (bind _returnvalue (UserInterface|CreateWidget "/Game/Content/UI/HUD.HUD_C" self))
      (bind _output_get (Variables|Default|SetHUD _returnvalue))
      (UserInterface|Viewport|AddtoViewport _output_get 0))
    (:else)))

(event Custom|GameEnd
  (Widget|RemovefromParent (Variables|Default|GetHUD))
  (bind _returnvalue (UserInterface|CreateWidget "/Game/Content/UI/UI_Last.UI_Last_C" self))
  (Variables|/Script/UMG.TextBlock|SetText (Variables|/Game/Content/UI/UI_Last.UI_Last_C|GetWho _returnvalue) (Utilities|Text|ToText(String) (CallFunction|DecideWho)))
  (UserInterface|Viewport|AddtoViewport _returnvalue 0)
  (Input|SetInputModeUIOnly self 0 "DoNotLock" false)
  (Variables|Default|SetbShowMouseCursor true))

(event Custom|UnFreeze
  (Widget|RemovefromParent (Variables|Default|GetCountDown))
  (Input|EnableInput (Pawn|GetControlledPawn) self))

(event Custom|CreateCountDown
  (Variables|Default|GetCountDown
    (:then
      (Default|StartTimer (Variables|Default|GetCountDown))
      (UserInterface|Viewport|AddtoViewport (Variables|Default|GetCountDown) 0))
    (:else
      (bind _returnvalue (UserInterface|CreateWidget "/Game/Content/UI/CountDown.CountDown_C" self))
      (bind _output_get (Variables|Default|SetCountDown _returnvalue))
      (UserInterface|Viewport|AddtoViewport _output_get 0))))

(event EventBeginPlay
  (bind _output_get (Variables|Default|SetbShowMouseCursor false))
  (Input|SetInputModeGameOnly self _output_get))

(fn ConstructionScript)

(fn DecideWho
  (if (== (Variables|Default|GetBlueScore) (Variables|Default|GetRedScore))
    (return "TIE")
    (elif (> (Variables|Default|GetBlueScore) (Variables|Default|GetRedScore))
      (return "Blue Wins")
      (else
        (return "Red Wins")))))

(fn OnRepBlueScore
  (bind _hud (Variables|Default|GetHUD)
    (:then
      (Variables|/Script/UMG.TextBlock|SetText (Variables|/Game/Content/UI/HUD.HUD_C|GetBlueScore _hud) (Utilities|Text|FormatText "Blue : {bluescore}" (Variables|Default|GetBlueScore))))
    (:else)))

(fn OnRepRedScore
  (bind _hud (Variables|Default|GetHUD)
    (:then
      (Variables|/Script/UMG.TextBlock|SetText (Variables|/Game/Content/UI/HUD.HUD_C|GetRedScore _hud) (Utilities|Text|FormatText "Red : {redscore}" (Variables|Default|GetRedScore))))
    (:else)))